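; Player character Blueprint for a 2D side-view game, handling horizontal movement, jumping and opening the pause menu.
; Horizontal axis input swaps the sprite between running and idle flipbooks based on velocity, rotates it to face the movement direction, and adds movement along X.
; Jump sets the jump velocity and plays a sound when not falling.
; The pause input pauses the game, shows the IngameMenu widget and enables the mouse cursor.
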(event Custom|UpdateAnimation
  ;[1 1 1] Animations for 2d char
  (Sprite|SetFlipbook (Variables|Default|GetSprite) (select (> (Math|Vector|VectorLength (Transformation|GetVelocity)) 0.0) "/Game/textures/sprites/pokemon/runningleft.runningleft" "/Game/textures/sprites/pokemon/idle.idle")))

(event Input|ActionEvents|InputActionPauseMenu
  ;[1 1 1] Pause Menu
  (:Pressed
    (Game|SetGamePaused true)
    (bind _returnvalue (UserInterface|CreateWidget "/Game/Blueprints/IngameMenu.IngameMenu_C"))
    (UserInterface|Viewport|AddtoViewport _returnvalue 0)
    (Variables|/Script/Engine.PlayerController|SetbShowMouseCursor (Game|GetPlayerController 0) true)))

(event Input|ActionEvents|InputActionJump
  (bind _charactermovement (Variables|Character|GetCharacterMovement))
  ;[1 1 1] Set jumping distance when doing first jump
  (:Pressed
    (Variables|/Script/Engine.CharacterMovementComponent|SetJumpZVelocity _charactermovement 525.0)
    (if (not (AI|Components|NavMovement|IsFalling _charactermovement))
      (Character|Jump)
      (Audio|PlaySound2D "/Game/Sounds/jumpsound.jumpsound")))
  (:Released
    (Character|StopJumping)))

(event Input|AxisEvents|InputAxisHorizontalMovement
  (params (AxisValue :type Float%20%28single-precision%29))
  (bind _sprite (Variables|Default|GetSprite))
  ;[1 1 1] Moving left and right
  (CallFunction|UpdateAnimation)
  (if (> AxisValue 0.0)
    (Transformation|SetRelativeRotation _sprite "0,180.000000, 0" false)
    (Pawn|Input|AddMovementInput "0.500000, 0, 0" AxisValue false :!label _label)
    (elif (< AxisValue 0.0)
      (Transformation|SetRelativeRotation _sprite "0,0.000000, 0" false)
      (goto _label))))

(fn ConstructionScript)